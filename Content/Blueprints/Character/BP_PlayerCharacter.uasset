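; Player character Blueprint that handles the visual side of first-person and full-body representations, including equipped weapon and torch.
; On BeginPlay it switches off the first-person torch's Niagara effect and shows either Mesh or FullBodyMesh based on local control.
; Equip events toggle the matching gun or torch by the same check.
; Weapon rarity sets the GunMesh material only, and the torch event activates Niagara even when unequipping.
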(event `self.ReceiveBeginPlay`
  (`ActorComponent.Deactivate` (`self.GetComponentByClass` (`ChildActorComponent.ChildActor` (`self.FirstPersonTorch`)) "/Script/Niagara.NiagaraComponent"))
  (if (`self.IsLocallyControlled`)
    (`SceneComponent.SetVisibility` (`self.FullBodyMesh`) false true)
    (`SceneComponent.SetVisibility` (`self.Mesh`) true false)
    (else
      (`SceneComponent.SetVisibility` (`self.FullBodyMesh`) true false)
      (`SceneComponent.SetVisibility` (`self.Mesh`) false false))))

(event `self.EquipWeaponGraphical`
  (params (bEquipWeapon :type Boolean) (WeaponRarity :type "EWeaponRarity Enum" :default "Common"))
  (bind _gun_mesh (`self.Gun Mesh`))
  (if (`self.IsLocallyControlled`)
    (`SceneComponent.SetVisibility` _gun_mesh bEquipWeapon false)
    (else
      (`SceneComponent.SetVisibility` (`self.FullBodyGunMesh`) bEquipWeapon false)))
  (switch `EWeaponRarity` WeaponRarity
    (:`Common`
      (`PrimitiveComponent.SetMaterial` _gun_mesh 0 "/Game/Materials/Pickups/CommonMaterial.CommonMaterial"))
    (:`Rare`
      (`PrimitiveComponent.SetMaterial` _gun_mesh 0 "/Game/Materials/Pickups/RareMaterial.RareMaterial"))
    (:`Master`
      (`PrimitiveComponent.SetMaterial` _gun_mesh 0 "/Game/Materials/Pickups/MasterMaterial.MasterMaterial"))
    (:`Legendary`
      (`PrimitiveComponent.SetMaterial` _gun_mesh 0 "/Game/Materials/Pickups/LegendaryMaterial.LegendaryMaterial"))))

(event `self.EquipTorchGraphical`
  (params (bEquipTorch :type Boolean) (bIsLit :type Boolean))
  (if (`self.IsLocallyControlled`)
    (`SceneComponent.SetVisibility` (`self.FirstPersonTorch`) bEquipTorch false)
    (`ActorComponent.Activate` (`self.GetComponentByClass` (`ChildActorComponent.ChildActor` (`self.FirstPersonTorch`)) "/Script/Niagara.NiagaraComponent") false)
    (else
      (`SceneComponent.SetVisibility` (`self.FullBodyTorch`) bEquipTorch false)
      (`ActorComponent.Activate` (`self.GetComponentByClass` (`ChildActorComponent.ChildActor` (`self.FullBodyTorch`)) "/Script/Niagara.NiagaraComponent") false))))

(fn `UserConstructionScript`)