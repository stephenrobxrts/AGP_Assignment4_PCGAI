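; Pedestal actor that displays four artefact pickups as child actors and shows which artefacts have been placed through their materials.
; On BeginPlay, every child pickup mesh receives a shared common material.
; UpdateVisibility maps each ArtefactsPlaced index to its child actor and applies that artefact's own material when the flag is true.
; It never reverts materials for false flags and still contains debug prints.
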(event `self.ReceiveBeginPlay`
  (for _array_element (`self.GetAllChildActors` false)
    (bind _asbp_artefact_pickup (cast `/Game/Blueprints/Pickups/BP_ArtefactPickup` _array_element))
    (`PrimitiveComponent.SetMaterial` (`PickupBase.PickupMesh` _asbp_artefact_pickup) 0 "/Game/Materials/Pickups/CommonMaterial.CommonMaterial")))

(event `self.UpdateVisibility`
  (`KismetSystemLibrary.PrintString` "UpdatingPedestal Visibility")
  (for (_array_element _array_index) (`self.ArtefactsPlaced`)
    (switch `int` _array_index
      (:`0`
        (bind _asbp_artefact_pickup (cast `/Game/Blueprints/Pickups/BP_ArtefactPickup` (`ChildActorComponent.ChildActor` (`self.BP_Artefact0`))))
        (if _array_element
          (bind _pickupmesh (`PickupBase.PickupMesh` _asbp_artefact_pickup))
          (`PrimitiveComponent.SetMaterial` _pickupmesh 0 "/Game/Materials/Pickups/ArtefactPickups/Artefact0.Artefact0")
          (`KismetSystemLibrary.PrintString` (`KismetStringLibrary.Conv_ObjectToString` (`PrimitiveComponent.GetMaterial` _pickupmesh 0)))))
      (:`1`
        (bind _asbp_artefact_pickup_2 (cast `/Game/Blueprints/Pickups/BP_ArtefactPickup` (`ChildActorComponent.ChildActor` (`self.BP_Artefact1`))))
        (if _array_element
          (`PrimitiveComponent.SetMaterial` (`PickupBase.PickupMesh` _asbp_artefact_pickup_2) 0 "/Game/Materials/Pickups/ArtefactPickups/Artefact1.Artefact1")))
      (:`2`
        (bind _asbp_artefact_pickup_3 (cast `/Game/Blueprints/Pickups/BP_ArtefactPickup` (`ChildActorComponent.ChildActor` (`self.BP_Artefact2`))))
        (if _array_element
          (`PrimitiveComponent.SetMaterial` (`PickupBase.PickupMesh` _asbp_artefact_pickup_3) 0 "/Game/Materials/Pickups/ArtefactPickups/Artefact2.Artefact2")))
      (:`3`
        (bind _asbp_artefact_pickup_4 (cast `/Game/Blueprints/Pickups/BP_ArtefactPickup` (`ChildActorComponent.ChildActor` (`self.BP_Artefact3`))))
        (if _array_element
          (`PrimitiveComponent.SetMaterial` (`PickupBase.PickupMesh` _asbp_artefact_pickup_4) 0 "/Game/Materials/Pickups/ArtefactPickups/Artefact3.Artefact3"))))))

(fn `UserConstructionScript`)