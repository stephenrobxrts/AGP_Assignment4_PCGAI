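; BP_Torch is a torch with a flickering point light, Niagara effect and looping-style audio cue, driven by its lit state.
; BeginPlay hides the Torch component, without its children, when held.
; Tick pauses the cue when hidden or unlit, toggles Niagara, and uses time-scaled Perlin noise to flicker the light's intensity, temperature and source radii.
; The node that would randomise flicker speed is never executed.
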(event `self.ReceiveBeginPlay`
  (bind _returnvalue (`self.GetIsHeld`))
  (`SceneComponent.SetVisibility` (`self.Torch`) (not _returnvalue) false))

(event `self.ReceiveTick`
  (params (DeltaSeconds :type "Float (single-precision)"))
  (bind _returnvalue (`KismetAnimationLibrary.K2_MakePerlinNoiseAndRemap` (* (`GameplayStatics.GetRealTimeSeconds`) (`self.Speed`)) 0.2 1.0))
  (`AudioComponent.SetPaused` (`self.TorchCue`) (or (not (`SceneComponent.bVisible` (`self.Torch`))) (not (`self.bIsLit`))))
  (if (`self.bIsLit`)
    (`ActorComponent.Activate` (`self.Niagara`) false)
    (`LightComponent.SetTemperature` (`self.PointLight`) (* 2700.0 (`KismetMathLibrary.FMax` _returnvalue 0.8)))
    (`LightComponent.SetIntensity` (`self.PointLight`) (* 200.0 _returnvalue))
    (`PointLightComponent.SetSourceRadius` (`self.PointLight`) (* 10.0 _returnvalue))
    (`PointLightComponent.SetSoftSourceRadius` (`self.PointLight`) (* 10.0 _returnvalue))
    (else
      (`LightComponent.SetIntensity` (`self.PointLight`) 0.0)
      (`ActorComponent.Deactivate` (`self.Niagara`)))))

(fn `UserConstructionScript`)