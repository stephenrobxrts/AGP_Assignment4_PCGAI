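; BP_TestTorch is a test torch actor whose point light flickers like a flame.
; Each Tick, it samples Perlin noise over real time and remaps it to a narrow multiplier range.
; That multiplier scales the light's temperature, intensity, source radius and soft source radius, so all four waver in sync.
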(event `self.ReceiveTick`
  (params (DeltaSeconds :type "Float (single-precision)"))
  (bind _returnvalue (`KismetAnimationLibrary.K2_MakePerlinNoiseAndRemap` (* (`GameplayStatics.GetRealTimeSeconds`) 5.0) 0.6 1.0))
  (`LightComponent.SetTemperature` (`self.PointLight`) (* 2700.0 _returnvalue))
  (`LightComponent.SetIntensity` (`self.PointLight`) (* 200.0 _returnvalue))
  (`PointLightComponent.SetSourceRadius` (`self.PointLight`) (* 10.0 _returnvalue))
  (`PointLightComponent.SetSoftSourceRadius` (`self.PointLight`) (* 10.0 _returnvalue)))

(fn `UserConstructionScript`)